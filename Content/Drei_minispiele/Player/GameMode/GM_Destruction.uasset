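; GM_Destruction is the game mode for a destruction minigame that decides when the player wins or loses.
; CheckWinCondition shows the win widget once enough good boxes are destroyed, while CheckLoseCondition shows the lose widget, meant for when the player explodes.
; Both outcomes share one end sequence that pauses the game, switches to UI-only input and shows the mouse cursor.
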(event Custom|CheckWinCondition
  (bind _returnvalue (Game|GetPlayerController 0))
  ;[0.15 0.15 0.15 0.5] Check if Player destroyed 2 good boxes
  (if (>= (Variables|Default|GetBoxesDestroyed) 2)
    (bind _returnvalue_2 (UserInterface|CreateWidget "/Game/Drei_minispiele/Widgets/Common/WG_Win.WG_Win_C"))
    (UserInterface|Viewport|AddtoViewport _returnvalue_2 0)
    (Game|SetGamePaused true)
    (Input|SetInputModeUIOnly _returnvalue 0 "DoNotLock" false)
    (Variables|/Script/Engine.PlayerController|SetbShowMouseCursor _returnvalue true)))

(event Custom|CheckLoseCondition
  (bind _returnvalue (Game|GetPlayerController 0))
  ;[0.15 0.15 0.15 0.5] Check if Player exploded
  (bind _returnvalue_2 (UserInterface|CreateWidget "/Game/Drei_minispiele/Widgets/Common/WG_Lose.WG_Lose_C"))
  (UserInterface|Viewport|AddtoViewport _returnvalue_2 0)
  (Game|SetGamePaused true)
  (Input|SetInputModeUIOnly _returnvalue 0 "DoNotLock" false)
  (Variables|/Script/Engine.PlayerController|SetbShowMouseCursor _returnvalue true))

(event EventBeginPlay)

(event EventTick
  (params (DeltaSeconds :type Float%20%28single-precision%29)))

(fn ConstructionScript)