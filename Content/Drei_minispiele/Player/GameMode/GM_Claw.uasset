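; Game mode for the claw machine minigame, showing the WG_Machine widget and running the timed claw-positioning phase.
; StartNewGame, triggered from BP_Pawn via the space bar, unlocks positioning and starts a looping timer that decrements PositionTimer.
; At zero it clears the timer and, through a DoOnce, locks the position and tells BP_Claw to run its down-up move.
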(event Custom|UpdateCountdown
  ;[0.15 0.15 0.15 0.5] Countdown for the timer to positionning the claw
  (if (not (Variables|Default|GetIsPositionLocked?))
    (bind _output_get (Variables|Default|SetPositionTimer (Math|Float|Clamp(Float) (- (Variables|Default|GetPositionTimer) 0.1) 0.0 1e+01)))
    (if (<= _output_get 0.0)
      (Utilities|Time|ClearandInvalidateTimerbyHandle (stale Custom|StartNewGame _output_get)) ; Reset timer
      ;;[0.15 0.15 0.15 0.5] If time <= 0  : Pos locked + get BP_Claw to tell him to go down by Event_ClawDown
      (Utilities|FlowControl|DoOnce false
        (:Completed
          (Variables|Default|SetIsPositionLocked? true)
          (bind _returnvalue (Actor|GetActorOfClass "/Game/Drei_minispiele/Blueprints/ClawMachine/BP_Claw.BP_Claw_C"))
          (Default|EventClawDownUp _returnvalue))))))

(event Custom|StartNewGame
  ;[0.15 0.15 0.15 0.5] Player can play when Espace Bar activated via BP_Pawn
  (Variables|Default|SetIsPlaying? true)
  (Variables|Default|SetIsPositionLocked? false)
  ;[0.15 0.15 0.15 0.5] Countdown for the timer to positionning the claw
  (bind _returnvalue (Utilities|Time|SetTimerbyEvent (delegate Custom|UpdateCountdown) 0.1 true))
  (bind _output_get (Variables|Default|SetTimer_ClawHandle _returnvalue)))

(event EventBeginPlay
  ;[0.15 0.15 0.15 0.5] Displays Widget claw machine
  (bind _returnvalue (UserInterface|CreateWidget "/Game/Drei_minispiele/Widgets/ClawMachine/WG_Machine.WG_Machine_C"))
  (UserInterface|Viewport|AddtoViewport _returnvalue 0))

(fn ConstructionScript)

(fn NewFunction)