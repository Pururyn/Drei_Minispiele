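; Player Blueprint for the destruction minigame, handling look, movement and attack through Enhanced Input.
; BeginPlay adds the player's mapping context; look input drives controller yaw and pitch.
; Movement follows the right and forward vectors of player controller 0's control rotation.
; The attack is a stub: a Visibility line trace with no start or end set and an unused result.
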(event Input|EnhancedActionEvents|EnhancedInputActionIA_Looking
  (params (ActionValue :type Vector%202D%20Structure) (ElapsedSeconds :type Float%20%28double-precision%29) (TriggeredSeconds :type Float%20%28double-precision%29) (InputAction :type Input%20Action%20Object%20Reference :default "/Game/Drei_minispiele/Player/Input_Action/IA_Looking.IA_Looking"))
  ;[0.15 0.15 0.15 0.5] Camera movement logic
  (Pawn|Input|AddControllerYawInput (.x ActionValue))
  (Pawn|Input|AddControllerPitchInput (.y ActionValue)))

(event Input|EnhancedActionEvents|EnhancedInputActionIA_Attacking
  (params (ActionValue :type Boolean) (ElapsedSeconds :type Float%20%28double-precision%29) (TriggeredSeconds :type Float%20%28double-precision%29) (InputAction :type Input%20Action%20Object%20Reference :default "/Game/Drei_minispiele/Player/Input_Action/IA_Attacking.IA_Attacking"))
  (Collision|LineTraceByChannel "0, 0, 0" "0, 0, 0" "TraceTypeQuery1" false 0 "None"))

(event Input|EnhancedActionEvents|EnhancedInputActionIA_Moving
  (params (ActionValue :type Vector%202D%20Structure) (ElapsedSeconds :type Float%20%28double-precision%29) (TriggeredSeconds :type Float%20%28double-precision%29) (InputAction :type Input%20Action%20Object%20Reference :default "/Game/Drei_minispiele/Player/Input_Action/IA_Moving.IA_Moving"))
  (bind _returnvalue (Game|GetPlayerController 0))
  (bind _returnvalue_2 (Pawn|GetControlRotation _returnvalue :!class /Script/Engine.Controller))
  (Pawn|Input|AddMovementInput (Math|Vector|GetRightVector _returnvalue_2) (.x ActionValue) false)
  (Pawn|Input|AddMovementInput (Math|Vector|GetForwardVector _returnvalue_2) (.y ActionValue) false))

(event EventBeginPlay
  ;[0.15 0.15 0.15 0.5] Get All player's action
  (Input|AddMappingContext (PlayerController|LocalPlayerSubsystems|GetEnhancedInputLocalPlayerSubsystem (Game|GetPlayerController 0)) "/Game/Drei_minispiele/Player/Input_Mapping_Context/IMC_DestructionPlayer.IMC_DestructionPlayer" 0 "(bIgnoreAllPressedKeysUntilRelease=True,bForceImmediately=False,bNotifyUserSettings=False)"))

(fn ConstructionScript)