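; Physics-driven claw for the claw machine minigame, moved sideways and dropped to grab goal objects.
; ApplyClawMovement receives a direction from BP_Pawn and sets it as the ClawSupport's linear velocity.
; Event_ClawDownUp animates the Rope constraint's Z limit with a timeline, pauses, then reverses and unlocks position in GM_Claw.
; Actors tagged Goal that hit the Claw are attached to it, keeping their world placement.
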(event OnComponentHit(Claw)
  (params (HitComponent :type Primitive%20Component%20Object%20Reference) (OtherActor :type Actor%20Object%20Reference) (OtherComp :type Primitive%20Component%20Object%20Reference) (NormalImpulse :type Vector :default "0, 0, 0") (Hit :type Hit%20Result%20Structure%20%28by%20ref%29))
  ;[0.15 0.15 0.15 0.5] Grab Object
  (if (Actor|ActorHasTag OtherActor "Goal")
    (Transformation|AttachComponentToComponent OtherActor (Variables|Default|GetClaw) "None" "KeepWorld" "KeepWorld" "KeepRelative" true)))

(event Custom|ApplyClawMovement
  (params (Direction :type Vector))
  ;[0.15 0.15 0.15 0.5] Get movement and condition from BP_Pawn
  (Physics|SetPhysicsLinearVelocity (Variables|Default|GetClaw_Support) Direction false "None"))

(event Custom|Event_ClawDownUp
  ;[0.15 0.15 0.15 0.5] Go down when time out of press space bar
  (bind (_direction _down) (Timeline|TL_ClawDownUp PlayFromStart)
    (:Update
      (Class|PhysicsConstraintComponent|SetLinearZLimit (Variables|Default|GetRope) "LCM_Limited" _down)
      ;[0.15 0.15 0.15 0.5] Wake up the claw
      (Class|PrimitiveComponent|WakeRigidBody (Variables|Default|GetClaw) "None"))
    (:Finished
      (if (Utilities|Enum|Equal(Enum) _direction "Backward")
        (bind _asgm_claw (Utilities|Casting|CastToGM_Claw (Game|GetGameMode)))
        (Variables|/Game/Drei_minispiele/Player/GameMode/GM_Claw.GM_Claw_C|SetIsPositionLocked? _asgm_claw false)
        (else
          (Utilities|FlowControl|Delay 1.0)
          (Timeline|TL_ClawDownUp Reverse))))))

(fn ConstructionScript)