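; Player pawn for the claw machine minigame that turns Enhanced Input movement into motion of the claw support.
; BeginPlay adds the IMC_Moving mapping context and finds the BP_Claw actor in the level.
; While IA_Moving triggers, it checks the GM_Claw game mode's position lock, then sends a scaled X/Y velocity to BP_Claw.
; Releasing the input sends a zero vector to stop the claw.
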(event Input|EnhancedActionEvents|EnhancedInputActionIA_Moving
  (params (ActionValue :type Vector%202D%20Structure) (ElapsedSeconds :type Float%20%28double-precision%29) (TriggeredSeconds :type Float%20%28double-precision%29) (InputAction :type Input%20Action%20Object%20Reference :default "/Game/Drei_minispiele/Player/Input_Action/IA_Moving.IA_Moving"))
  (bind (_x _y) (Math|Vector2D|BreakVector2D ActionValue))
  (:Triggered
    ;[0.15 0.15 0.15 0.5] Security to verify if the player can move the claw support or not
    (bind _asgm_claw (Utilities|Casting|CastToGM_Claw (Game|GetGameMode)))
    (if (not (Variables|/Game/Drei_minispiele/Player/GameMode/GM_Claw.GM_Claw_C|GetIsPositionLocked? _asgm_claw))
      ;[0.15 0.15 0.15 0.5] Send info to BP_Claw
      (Default|ApplyClawMovement (Variables|Default|GetClaw_Ref) (Math|Vector|MakeVector (* 5e+02 _x) (* _y -5e+02) 0.0))))
  (:Completed
    ;[0.15 0.15 0.15 0.5] Send to BP_Claw a stop moving when stop moving
    (Default|ApplyClawMovement (Variables|Default|GetClaw_Ref) "0, 0, 0")))

(event EventBeginPlay
  ;[0.15 0.15 0.15 0.5] Get the IMC_Moving to sent it to Claw
  (Input|AddMappingContext (PlayerController|LocalPlayerSubsystems|GetEnhancedInputLocalPlayerSubsystem (Game|GetPlayerController 0)) "/Game/Drei_minispiele/Player/Input_Mapping_Context/IMC_Moving.IMC_Moving" 0 "(bIgnoreAllPressedKeysUntilRelease=True,bForceImmediately=False,bNotifyUserSettings=False)")
  (bind _returnvalue (Actor|GetActorOfClass "/Game/Drei_minispiele/Blueprints/ClawMachine/BP_Claw.BP_Claw_C"))
  (Variables|Default|SetClaw_Ref _returnvalue))

(fn ConstructionScript)