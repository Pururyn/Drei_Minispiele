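; Lose trigger actor for the claw machine minigame that ends the game with a lose screen.
; When an actor overlaps its BoxLose collision, it loses if that actor is tagged "Lose" or the GM_Claw game mode has no credit left.
; On a loss it shows the WG_Lose widget, pauses the game, switches to UI-only input and shows the mouse cursor.
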(event OnComponentBeginOverlap(BoxLose)
  (params (OverlappedComponent :type Primitive%20Component%20Object%20Reference) (OtherActor :type Actor%20Object%20Reference) (OtherComp :type Primitive%20Component%20Object%20Reference) (OtherBodyIndex :type Integer) (bFromSweep :type Boolean) (SweepResult :type Hit%20Result%20Structure%20%28by%20ref%29))
  (bind _returnvalue (Game|GetPlayerController 0))
  ;[0.15 0.15 0.15 0.5] If Object with tag Lose touch the collision box OR if tag Goal don't touch BP_winM-> pop Lose Widget
  (bind _asgm_claw (Utilities|Casting|CastToGM_Claw (Game|GetGameMode)))
  (if (or (Actor|ActorHasTag OtherActor "Lose") (== (Variables|/Game/Drei_minispiele/Player/GameMode/GM_Claw.GM_Claw_C|GetCurrentCredit _asgm_claw) 0))
    (bind _returnvalue_2 (UserInterface|CreateWidget "/Game/Drei_minispiele/Widgets/Common/WG_Lose.WG_Lose_C"))
    (UserInterface|Viewport|AddtoViewport _returnvalue_2 0)
    (Game|SetGamePaused true)
    (Input|SetInputModeUIOnly _returnvalue 0 "DoNotLock" false)
    (Variables|/Script/Engine.PlayerController|SetbShowMouseCursor _returnvalue true)))

(fn ConstructionScript)