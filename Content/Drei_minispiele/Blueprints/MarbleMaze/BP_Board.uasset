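; BP_Board is the tiltable board of the MarbleMaze minigame, rotated by player input.
; On BeginPlay it adds the IMC_Moving mapping context to the first player's Enhanced Input subsystem.
; Each IA_Moving event turns the 2D input into a clamped-range roll and pitch target with zero yaw.
; The actor eases toward that target with RInterpTo, advancing only when the input event fires.
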(event Input|EnhancedActionEvents|EnhancedInputActionIA_Moving
  (params (ActionValue :type Vector%202D%20Structure) (ElapsedSeconds :type Float%20%28double-precision%29) (TriggeredSeconds :type Float%20%28double-precision%29) (InputAction :type Input%20Action%20Object%20Reference :default "/Game/Drei_minispiele/Player/Input_Action/IA_Moving.IA_Moving"))
  ;[0.15 0.15 0.15 0.5] BoardRotation by using Z/Q/S/D or Up/Down/Right/Left
  (Transformation|SetActorRotation (Math|Interpolation|RInterpTo (Transformation|GetActorRotation) (Math|Rotator|MakeRotator (* (.x ActionValue) 15.0) (* (.y ActionValue) -15.0) 0.0) (Utilities|Time|GetWorldDeltaSeconds) 3.0)))

(event EventBeginPlay
  ;[0.15 0.15 0.15 0.5] Get controller
  (Input|AddMappingContext (PlayerController|LocalPlayerSubsystems|GetEnhancedInputLocalPlayerSubsystem (Game|GetPlayerController 0)) "/Game/Drei_minispiele/Player/Input_Mapping_Context/IMC_Moving.IMC_Moving" 0 "(bIgnoreAllPressedKeysUntilRelease=True,bForceImmediately=False,bNotifyUserSettings=False)"))

(fn ConstructionScript)